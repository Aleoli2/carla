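; CARLA actor factory that publishes vehicle definitions built from its Vehicles list and spawns vehicles from actor descriptions.
; SpawnActor validates the class, spawns at the given transform, and reports success, collision or invalid description.
; Both BaseVehiclePawn and BaseVehiclePawnNW vehicles get a default WheeledVehicleAIController, with sticky control and body color read from the description's variation attributes, falling back to defaults.
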(fn `GenerateDefinitions`
  (returns (ReturnValue :type "Array of ActorDefinition Structure"))
  (bind _definitions (`ActorBlueprintFunctionLibrary.MakeVehicleDefinitions` (`self.Vehicles`)))
  (return _definitions))

(fn `SpawnActor`
  (params (SpawnAtTransform :type "Transform Structure (by ref)") (ActorDescription :type "ActorDescription Structure (by ref)"))
  (returns (SpawnResult :type "ActorSpawnResult Structure"))
  (locals (DefaultColor :type "Color Structure" :default (struct :`B` 231 :`R` 255)))
  (if (`KismetSystemLibrary.IsValidClass` ActorDescription_Class)
    (bind _returnvalue (`|SpawnActorFromClass` ActorDescription_Class SpawnAtTransform "Undefined" "OverrideRootScale" null null))
    (`/Engine/EditorBlueprintResources/StandardMacros.IsValid` _returnvalue
      (:`Is Valid`
        (bind _returnvalue_2 (`ActorBlueprintFunctionLibrary.RetrieveActorAttributeToColor` "color" ActorDescription_Variations (`local.DefaultColor`)))
        (bind _asbase_vehicle_pawn (cast `/Game/Carla/Blueprints/Vehicles/BaseVehiclePawn` _returnvalue)
          (:`then`
            (bind _instigator (`Actor.Instigator` _returnvalue))
            (`Pawn.SpawnDefaultController` _instigator)
            (bind _aswheeled_vehicle_aicontroller (cast `WheeledVehicleAIController` (`Pawn.GetController` _asbase_vehicle_pawn)))
            (bind _returnvalue_3 (`ActorBlueprintFunctionLibrary.RetrieveActorAttributeToBool` "sticky_control" ActorDescription_Variations true))
            (`WheeledVehicleAIController.SetStickyControl` _aswheeled_vehicle_aicontroller _returnvalue_3)
            (bind _returnvalue_4 (`KismetMathLibrary.Conv_ColorToLinearColor` _returnvalue_2))
            (`/Game/Carla/Blueprints/Vehicles/BaseVehiclePawn.ApplyColor` _asbase_vehicle_pawn _returnvalue_4)
            (return (make `ActorSpawnResult` _returnvalue "Success")))
          (:`CastFailed`
            (bind _asbase_vehicle_pawn_nw (cast `/Game/Carla/Blueprints/Vehicles/BaseVehiclePawnNW` _returnvalue))
            (`Pawn.SpawnDefaultController` _instigator)
            (bind _aswheeled_vehicle_aicontroller_2 (cast `WheeledVehicleAIController` (`Pawn.GetController` _asbase_vehicle_pawn_nw)))
            (bind _returnvalue_5 (`ActorBlueprintFunctionLibrary.RetrieveActorAttributeToBool` "sticky_control" ActorDescription_Variations true))
            (`WheeledVehicleAIController.SetStickyControl` _aswheeled_vehicle_aicontroller_2 _returnvalue_5)
            (`/Game/Carla/Blueprints/Vehicles/BaseVehiclePawnNW.ApplyColor` _asbase_vehicle_pawn_nw _returnvalue_4)
            (return (make `ActorSpawnResult` _returnvalue "Success")))))
      (:`Is Not Valid`
        (return (make `ActorSpawnResult` null "Collision"))))
    (else
      (return (make `ActorSpawnResult` null "InvalidDescription")))))

(fn `UserConstructionScript`)